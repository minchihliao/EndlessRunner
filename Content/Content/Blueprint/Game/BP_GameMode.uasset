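; Game mode that procedurally builds a branching road from random straight, curve and turn segments, preloading several at BeginPlay.
; Segments chain from stored end points in a runtime queue; after a turn, both branches grow in parallel without further turns for a set count.
; GetNextPath picks the path index from the turn input, updates player status on a missed turn, and on non-turn segments destroys passed or unchosen roads and spawns more.
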(event Custom|ReleaseRegion
  (bind _runtimeregionqueue (Variables|Default|GetRuntimeRegionQueue))
  (Utilities|Array|RemoveIndex _runtimeregionqueue)
  (Development|PrintString (Utilities|String|ToString(Vector) (.Location (Utilities|Struct|BreakS_Point (Utilities|Array|Get(acopy) (Variables|/Game/Content/Blueprint/Game/Course/BP_Road_Base.BP_Road_Base_C|GetPoints (Utilities|Array|Get(acopy) _runtimeregionqueue))))))))

(event EventBeginPlay
  (for _index (range 0 3)
    (CallFunction|SpwanRegion)))

(event EventTick
  (params (DeltaSeconds :type Float%20%28single-precision%29)))

(fn ConstructionScript)

(fn GetCurrentRoad
  (return (Utilities|Array|Get(acopy) (Variables|Default|GetRuntimeRegionQueue))))

(fn DequeueRegion
  (params (targetDirection :type E_Direction%20Enum :default "NewEnumerator0"))
  (bind _runtimeregionqueue (Variables|Default|GetRuntimeRegionQueue))
  (bind _runtimeregionqueue_2 (Variables|Default|GetRuntimeRegionQueue))
  (bind _runtimeregionqueue_3 (Variables|Default|GetRuntimeRegionQueue))
  (LocalVariables|SetPrevRoad (Utilities|Array|Get(acopy) _runtimeregionqueue_2))
  (Utilities|Array|RemoveIndex _runtimeregionqueue_2)
  (Actor|DestroyActor (LocalVariables|GetPrevRoad))
  (if (not (Utilities|Enum|Equal(Enum) targetDirection "NewEnumerator0"))
    (if (Utilities|Enum|Equal(Enum) targetDirection "NewEnumerator1")
      (for _index (range 0 (- (/ (Utilities|Array|Length (Variables|Default|GetRuntimeRegionQueue)) 2) 0))
        (LocalVariables|SetPrevRoad (Utilities|Array|Get(acopy) _runtimeregionqueue_3 (- (+ (* _index 2) 1) _index)))
        (Utilities|Array|RemoveIndex _runtimeregionqueue_3 (- (+ (* _index 2) 1) _index))
        (Actor|DestroyActor (LocalVariables|GetPrevRoad)))
      (Utilities|Array|RemoveIndex (Variables|Default|GetSpwanPoints) 1)
      (else
        (for _index_2 (range 0 (- (/ (Utilities|Array|Length (Variables|Default|GetRuntimeRegionQueue)) 2) 0))
          (LocalVariables|SetPrevRoad (Utilities|Array|Get(acopy) _runtimeregionqueue (- (* _index_2 2) _index_2)))
          (Utilities|Array|RemoveIndex _runtimeregionqueue (- (* _index_2 2) _index_2))
          (Actor|DestroyActor (LocalVariables|GetPrevRoad)))
        (Utilities|Array|RemoveIndex (Variables|Default|GetSpwanPoints))))))

(fn GetNextPath
  (params (IsTurnRegion :type Boolean) (TurnDirection :type E_Direction%20Enum%20%28by%20ref%29 :default "NewEnumerator0") (current%20direction :type E_Direction%20Enum :default "NewEnumerator0"))
  (LocalVariables|SetPlayerTurnDirection TurnDirection)
  ;[1 1 1] Current Region is turn region
  (if IsTurnRegion
    (if (Utilities|Enum|Equal(Enum) (LocalVariables|GetPlayerTurnDirection) "NewEnumerator0")
      ;;[1 1 1] No Turn
      (LocalVariables|SetPointsIndex "NewEnumerator3")
      (bind _asbp_game_state (Utilities|Casting|CastToBP_GameState (Game|GetGameState)))
      (Variables|/Game/Content/Blueprint/Game/BP_GameState.BP_GameState_C|SetPlayerStatus _asbp_game_state "NewEnumerator2")
      (else
        ;;[1 1 1] Turn
        (if (Utilities|Enum|Equal(Enum) (LocalVariables|GetPlayerTurnDirection) "NewEnumerator2")
          (LocalVariables|SetPointsIndex "NewEnumerator2")
          (else
            (LocalVariables|SetPointsIndex "NewEnumerator1")))))
    (Default|CallPassRegionDispatchers)
    (|SetBy-RefVar TurnDirection "NewEnumerator0")
    (return (LocalVariables|GetPointsIndex))
    (else
      ;[1 1 1] Current Region is Not turn region
      (CallFunction|DequeueRegion current%20direction)
      (CallFunction|SpwanRegion)
      (LocalVariables|SetPointsIndex "NewEnumerator0")
      (Default|CallPassRegionDispatchers)
      (|SetBy-RefVar TurnDirection "NewEnumerator0")
      (return (LocalVariables|GetPointsIndex)))))

(fn SpwanRegion
  (if (<= (Variables|Default|GetRemainRegion) 0)
    (bind _returnvalue (Game|SpawnActorfromClass (Utilities|Select :Index (Math|Random|RandomIntegerinRange 0 2) :Option%200 "/Game/Content/Blueprint/Game/Course/BP_Road_Straight.BP_Road_Straight_C" :Option%201 "/Game/Content/Blueprint/Game/Course/BP_Road_Curve.BP_Road_Curve_C" :Option%202 "/Game/Content/Blueprint/Game/Course/BP_Road_Turn.BP_Road_Turn_C") (Math|Transform|MakeTransform (.Location (Utilities|Struct|BreakS_Point (Utilities|Array|Get(acopy) (Variables|Default|GetSpwanPoints)))) "0, 0, 0" "1.000000,1.000000,1.000000") "Undefined" 0 0))
    (Transformation|AddWorldRotation (Variables|/Script/Engine.Actor|GetRootComponent _returnvalue) (.Rotator (Utilities|Struct|BreakS_Point (Utilities|Array|Get(acopy) (Variables|Default|GetSpwanPoints)))) false false)
    (bind _asbp_road_base (Utilities|Casting|CastToBP_Road_Base _returnvalue))
    (bind _asbp_road_turn (Utilities|Casting|CastToBP_Road_Turn _asbp_road_base)
      (:then
        (Default|SetAllPoints _asbp_road_turn)
        (Utilities|Array|Add (Variables|Default|GetRuntimeRegionQueue) _asbp_road_base)
        (Variables|Default|SetSpwanPoints (Utilities|Array|MakeArray (Utilities|Array|Get(acopy) (Utilities|Struct|BreakS_AllRegionPoints (Utilities|Array|Get(acopy) (Variables|/Game/Content/Blueprint/Game/Course/BP_Road_Base.BP_Road_Base_C|GetAllPoints _asbp_road_base) 1)) (- (Utilities|Array|Length (Utilities|Struct|BreakS_AllRegionPoints (Utilities|Array|Get(acopy) (Variables|/Game/Content/Blueprint/Game/Course/BP_Road_Base.BP_Road_Base_C|GetAllPoints _asbp_road_base) 1))) 1)) (Utilities|Array|Get(acopy) (Utilities|Struct|BreakS_AllRegionPoints (Utilities|Array|Get(acopy) (Variables|/Game/Content/Blueprint/Game/Course/BP_Road_Base.BP_Road_Base_C|GetAllPoints _asbp_road_base) 2)) (- (Utilities|Array|Length (Utilities|Struct|BreakS_AllRegionPoints (Utilities|Array|Get(acopy) (Variables|/Game/Content/Blueprint/Game/Course/BP_Road_Base.BP_Road_Base_C|GetAllPoints _asbp_road_base) 2))) 1))))
        (Variables|Default|SetRemainRegion (* (Variables|Default|GetPreLoadRegionNumber) 2)))
      (:CastFailed
        (bind _asbp_road_base_2 (Utilities|Casting|CastToBP_Road_Base _asbp_road_base))
        (Default|SetAllPoints _asbp_road_base_2)
        (Utilities|Array|Add (Variables|Default|GetRuntimeRegionQueue) _asbp_road_base_2)
        (Variables|Default|SetSpwanPoints (Utilities|Array|MakeArray (Utilities|Array|Get(acopy) (Utilities|Struct|BreakS_AllRegionPoints (Utilities|Array|Get(acopy) (Variables|/Game/Content/Blueprint/Game/Course/BP_Road_Base.BP_Road_Base_C|GetAllPoints _asbp_road_base_2))) (- (Utilities|Array|Length (Utilities|Struct|BreakS_AllRegionPoints (Utilities|Array|Get(acopy) (Variables|/Game/Content/Blueprint/Game/Course/BP_Road_Base.BP_Road_Base_C|GetAllPoints _asbp_road_base_2)))) 1))))))
    (else
      (bind _returnvalue_2 (Game|SpawnActorfromClass (Utilities|Select :Index (Math|Random|RandomIntegerinRange 0 1) :Option%200 "/Game/Content/Blueprint/Game/Course/BP_Road_Straight.BP_Road_Straight_C" :Option%201 "/Game/Content/Blueprint/Game/Course/BP_Road_Curve.BP_Road_Curve_C" :Option%202 "/Game/Content/Blueprint/Game/Course/BP_Road_Turn.BP_Road_Turn_C") (Math|Transform|MakeTransform (.Location (Utilities|Struct|BreakS_Point (Utilities|Array|Get(acopy) (Variables|Default|GetSpwanPoints)))) "0, 0, 0" "1.000000,1.000000,1.000000") "Undefined" 0 0))
      (LocalVariables|SetRightRegion _returnvalue_2)
      (Transformation|AddWorldRotation (Variables|/Script/Engine.Actor|GetRootComponent _returnvalue_2) (.Rotator (Utilities|Struct|BreakS_Point (Utilities|Array|Get(acopy) (Variables|Default|GetSpwanPoints)))) false false)
      (bind _returnvalue_3 (Game|SpawnActorfromClass (Utilities|Select :Index (Math|Random|RandomIntegerinRange 0 1) :Option%200 "/Game/Content/Blueprint/Game/Course/BP_Road_Straight.BP_Road_Straight_C" :Option%201 "/Game/Content/Blueprint/Game/Course/BP_Road_Curve.BP_Road_Curve_C" :Option%202 "/Game/Content/Blueprint/Game/Course/BP_Road_Turn.BP_Road_Turn_C") (Math|Transform|MakeTransform (.Location (Utilities|Struct|BreakS_Point (Utilities|Array|Get(acopy) (Variables|Default|GetSpwanPoints) 1))) "0, 0, 0" "1.000000,1.000000,1.000000") "Undefined" 0 0))
      (LocalVariables|SetLeftRegion _returnvalue_3)
      (Development|PrintString (Utilities|String|ToString(Vector) (.Location (Utilities|Struct|BreakS_Point (Utilities|Array|Get(acopy) (Variables|Default|GetSpwanPoints) 1)))))
      (Transformation|AddWorldRotation (Variables|/Script/Engine.Actor|GetRootComponent _returnvalue_3) (.Rotator (Utilities|Struct|BreakS_Point (Utilities|Array|Get(acopy) (Variables|Default|GetSpwanPoints) 1))) false false)
      (bind _asbp_road_base_3 (Utilities|Casting|CastToBP_Road_Base (LocalVariables|GetRightRegion)))
      (Default|SetAllPoints _asbp_road_base_3)
      (bind _asbp_road_base_4 (Utilities|Casting|CastToBP_Road_Base (LocalVariables|GetRightRegion)))
      (Utilities|Array|Add (Variables|Default|GetRuntimeRegionQueue) _asbp_road_base_3)
      (Variables|Default|SetSpwanPoints (Utilities|Array|MakeArray (Utilities|Array|Get(acopy) (Utilities|Struct|BreakS_AllRegionPoints (Utilities|Array|Get(acopy) (Variables|/Game/Content/Blueprint/Game/Course/BP_Road_Base.BP_Road_Base_C|GetAllPoints _asbp_road_base_4))) (- (Utilities|Array|Length (Utilities|Struct|BreakS_AllRegionPoints (Utilities|Array|Get(acopy) (Variables|/Game/Content/Blueprint/Game/Course/BP_Road_Base.BP_Road_Base_C|GetAllPoints _asbp_road_base_4)))) 1))))
      (bind _asbp_road_base_5 (Utilities|Casting|CastToBP_Road_Base (LocalVariables|GetLeftRegion)))
      (Default|SetAllPoints _asbp_road_base_5)
      (bind _asbp_road_base_6 (Utilities|Casting|CastToBP_Road_Base (LocalVariables|GetLeftRegion)))
      (Utilities|Array|Add (Variables|Default|GetRuntimeRegionQueue) _asbp_road_base_5)
      (Utilities|Array|Add (Variables|Default|GetSpwanPoints) (Utilities|Array|Get(acopy) (Utilities|Struct|BreakS_AllRegionPoints (Utilities|Array|Get(acopy) (Variables|/Game/Content/Blueprint/Game/Course/BP_Road_Base.BP_Road_Base_C|GetAllPoints _asbp_road_base_6))) (- (Utilities|Array|Length (Utilities|Struct|BreakS_AllRegionPoints (Utilities|Array|Get(acopy) (Variables|/Game/Content/Blueprint/Game/Course/BP_Road_Base.BP_Road_Base_C|GetAllPoints _asbp_road_base_6)))) 1)))
      (Variables|Default|SetRemainRegion (- (Variables|Default|GetRemainRegion) 2)))))