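; Game state Blueprint that tracks the player's status, score and current road region.
; On BeginPlay it sets the initial status, starts a looping timer that steadily raises the score, and binds to the game mode's pass-region dispatchers.
; At start and whenever that dispatcher fires, it caches the game mode's current road as the current region.
; IsCrossroad is a stub that always returns false.
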(event Custom|IncreaseScore
  (Variables|Default|SetScore (+ (Variables|Default|GetScore) 2)))

(event Custom|PassRegionDispatchers_Event
  (CallFunction|SetCurrentRegion))

(event EventBeginPlay
  (Variables|Default|SetPlayerStatus "NewEnumerator0")
  (bind _returnvalue (Utilities|Time|SetTimerbyFunctionName 0 "IncreaseScore" 0.05 true))
  (Variables|Default|SetScoreTimer _returnvalue)
  (bind _asbp_game_mode (Utilities|Casting|CastToBP_GameMode (Game|GetGameMode)))
  (bind _output_get (Variables|Default|SetGameModeRef _asbp_game_mode))
  (EventDispatchers|AssignPassRegionDispatchers _output_get (delegate Custom|PassRegionDispatchers_Event))
  (CallFunction|SetCurrentRegion))

(event EventTick
  (params (DeltaSeconds :type Float%20%28single-precision%29)))

(fn ConstructionScript)

(fn GetCurrentRegion
  (return (Variables|Default|GetCurrentRegion)))

(fn SetCurrentRegion
  (bind _output (Default|GetCurrentRoad (Variables|Default|GetGameModeRef)))
  (Variables|Default|SetCurrentRegion _output))

(fn IsCrossroad
  (return false))