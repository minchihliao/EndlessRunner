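; Endless-runner player character that auto-runs along road-region waypoints, with Space to jump and an end screen on hitting an obstacle.
; Tick runs UpdatePlayer1, steering through target points via a virtual PlayerPosition, separate from the actor's held A/D sidestep.
; When points run out, OnPassRegion gets the next path from the GameMode, using Q/E turns registered near the region's end.
; Older update and move variants remain unused.
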(event EventBeginPlay
  (bind _asbp_game_mode (Utilities|Casting|CastToBP_GameMode (Game|GetGameMode)))
  (Variables|Default|SetGameModeRef _asbp_game_mode)
  (bind _asbp_game_state (Utilities|Casting|CastToBP_GameState (Game|GetGameState)))
  (Variables|Default|SetGameStateRef _asbp_game_state)
  (Variables|Default|Setspeed (Variables|/Game/Content/Blueprint/Game/BP_GameState.BP_GameState_C|GetPlayerSpeed (Variables|Default|GetGameStateRef)))
  (CallFunction|SetCurrentRoad "NewEnumerator0")
  (bind _targetpoints (Default|GetRegionTargetPoints (.Region (Utilities|Struct|BreakS_PlayerCurrentRegion (Variables|Default|GetNewCurrentRegion))) "NewEnumerator0"))
  (Variables|Default|SetTargetPoints _targetpoints)
  (Variables|Default|SetPlayerPosition "0, 0, 0"))

(event Collision|EventHit
  (params (MyComp :type Primitive%20Component%20Object%20Reference) (Other :type Actor%20Object%20Reference) (OtherComp :type Primitive%20Component%20Object%20Reference) (bSelfMoved :type Boolean) (HitLocation :type Vector :default "0, 0, 0") (HitNormal :type Vector :default "0, 0, 0") (NormalImpulse :type Vector :default "0, 0, 0") (Hit :type Hit%20Result%20Structure%20%28by%20ref%29))
  (Utilities|Casting|CastToObstacle_BASE Other)
  (Utilities|FlowControl|DoOnce false
    (:Completed
      (bind _returnvalue (UserInterface|CreateWidget "/Game/Content/UI/EndScreen.EndScreen_C"))
      (UserInterface|Viewport|AddtoViewport _returnvalue 0))))

(event EventTick
  (params (DeltaSeconds :type Float%20%28single-precision%29))
  (CallFunction|UpdatePlayer1 DeltaSeconds))

(event Input|KeyboardEvents|SpaceBar
  (params (Key :type Key%20Structure :default "None"))
  (:Pressed
    (Character|Jump)
    (Variables|Default|SetJumping true))
  (:Released
    (Character|StopJumping)
    (Variables|Default|SetJumping false)))

(event Input|KeyboardEvents|Q
  (params (Key :type Key%20Structure :default "None"))
  (:Pressed
    (CallFunction|Turn "NewEnumerator2")))

(event Input|KeyboardEvents|E
  (params (Key :type Key%20Structure :default "None"))
  (:Pressed
    (CallFunction|Turn "NewEnumerator1")))

(event Input|KeyboardEvents|A
  (params (Key :type Key%20Structure :default "None"))
  (:Pressed
    (Class|Actor|AddActorLocalTransform (Math|Transform|MakeTransform (* "0.000000,1.000000,0.000000" "0.000000,-450.000000,0.000000") "0, 0, 0" "1.000000,1.000000,1.000000") false false))
  (:Released
    (Class|Actor|AddActorLocalTransform (Math|Transform|MakeTransform (* "0.000000,1.000000,0.000000" "0.000000,450.000000,0.000000") "0, 0, 0" "1.000000,1.000000,1.000000") false false)))

(event Input|KeyboardEvents|D
  (params (Key :type Key%20Structure :default "None"))
  (:Pressed
    (Class|Actor|AddActorLocalTransform (Math|Transform|MakeTransform (* "0.000000,1.000000,0.000000" "0.000000,450.000000,0.000000") "0, 0, 0" "1.000000,1.000000,1.000000") false false))
  (:Released
    (Class|Actor|AddActorLocalTransform (Math|Transform|MakeTransform (* "0.000000,1.000000,0.000000" "0.000000,-450.000000,0.000000") "0, 0, 0" "1.000000,1.000000,1.000000") false false)))

(fn ConstructionScript)

(fn SetCurrentRoad
  (params (Current%20Path :type E_Direction%20Enum :default "NewEnumerator0"))
  (bind _currentregion (Default|GetCurrentRegion (Variables|Default|GetGameStateRef)))
  (Variables|Default|SetNewCurrentRegion (Utilities|Struct|MakeS_PlayerCurrentRegion _currentregion Current%20Path)))

(fn CharactorMove
  (params (DeltaTime :type Float%20%28single-precision%29) (direction :type Vector) (rotator :type Rotator))
  (bind _returnvalue (Transformation|GetActorRotation))
  (bind _returnvalue_2 (* _returnvalue -1.0))
  (bind _returnvalue_3 (Math|Rotator|CombineRotators rotator _returnvalue_2))
  (bind _returnvalue_4 (Math|Rotator|MakeRotator (.roll _returnvalue_3) (.pitch _returnvalue_3) (.yaw _returnvalue_3)))
  (Transformation|AddActorLocalOffset (* (Math|Vector|Normalize direction) (* DeltaTime (Variables|Default|Getspeed))) false false)
  (LocalVariables|SetActor%20Rotation _returnvalue_2)
  (LocalVariables|SetCharactorRotator _returnvalue_4)
  (Variables|Default|SetCharactor _returnvalue_4)
  (LocalVariables|SetMeshRotator (Math|Rotator|CombineRotators rotator (* (Math|Rotator|CombineRotators (Transformation|GetWorldRotation (Variables|Character|GetMesh)) "0.000000,90.000000,0.000000") -1.0)))
  (if (>= (Math|Float|Absolute(Float) (.yaw _returnvalue_3)) 1e+01)
    (Transformation|AddActorLocalRotation (LocalVariables|GetCharactorRotator) false false)
    (Transformation|SetRelativeRotation (Variables|Character|GetMesh) "0.000000,-90.000000,0.000000" false false)
    (else
      (Transformation|AddLocalRotation (Variables|Character|GetMesh) (LocalVariables|GetMeshRotator) false false))))

(fn UpdatePlayer
  (params (delta%20Seconds :type Float%20%28double-precision%29))
  (bind _returnvalue (Transformation|GetActorLocation))
  (bind _targetpoints (Variables|Default|GetTargetPoints))
  (if (Utilities|IsValid (.Region (Utilities|Struct|BreakS_PlayerCurrentRegion (Variables|Default|GetNewCurrentRegion))))
    (if (Utilities|Array|IsEmpty (Variables|Default|GetTargetPoints))
      (if (Utilities|Enum|NotEqual(Enum) (Variables|/Game/Content/Blueprint/Game/BP_GameState.BP_GameState_C|GetPlayerStatus (Variables|Default|GetGameStateRef)) "NewEnumerator2")
        (CallFunction|OnPassRegion)
        (else
          (Variables|Default|SetNewCurrentRegion "")
          (Utilities|Array|Clear (Variables|Default|GetTargetPoints))
          (Development|PrintString "Died")))
      (else
        (bind _output_get (LocalVariables|SetnexPoint (Utilities|Array|Get(acopy) (Variables|Default|GetTargetPoints))))
        (LocalVariables|SetStartPosition _returnvalue)
        (LocalVariables|SetTargetPosition (+ (.Location (Utilities|Struct|BreakS_Point _output_get)) "0.000000,0.000000,92.802551"))
        (bind _output_get_2 (LocalVariables|SetmoveDistance (Math|Vector|Distance(Vector) _returnvalue (+ (.Location (Utilities|Struct|BreakS_Point _output_get)) "0.000000,0.000000,92.802551"))))
        (LocalVariables|Setdirection (- (+ (.Location (Utilities|Struct|BreakS_Point _output_get)) "0.000000,0.000000,92.802551") (Transformation|GetActorLocation)))
        (if (> _output_get_2 (* delta%20Seconds (Variables|Default|Getspeed)))
          (CallFunction|CharactorMove delta%20Seconds (LocalVariables|Getdirection) (Math|Rotator|FindLookatRotation (LocalVariables|GetStartPosition) (LocalVariables|GetTargetPosition)))
          (else
            (Development|PrintString (Utilities|String|ToString(Vector) (.Location (Utilities|Struct|BreakS_Point (Utilities|Array|Get(acopy) _targetpoints)))))
            (Utilities|Array|RemoveIndex _targetpoints)
            (Transformation|AddActorLocalRotation (Variables|Default|GetCharactor) false false)
            (Transformation|SetRelativeRotation (Variables|Character|GetMesh) "0.000000,-90.000000,0.000000" false false)))))))

(fn OnPassRegion
  (bind _turndirection (Variables|Default|GetTurnDirection))
  (bind _newcurrentregion (Variables|Default|GetNewCurrentRegion))
  (bind _bsuccess (Utilities|Casting|CastToBP_Road_Turn (.region _newcurrentregion)))
  (bind _returnvalue (Utilities|Enum|Equal(Enum) (.currentpath _newcurrentregion) "NewEnumerator0"))
  (bind _output_get (LocalVariables|SetIsCrossRoad (and _bsuccess _returnvalue)))
  (Development|PrintString (Utilities|String|Append (Utilities|String|ToString(Boolean) _bsuccess) (Utilities|String|ToString(Boolean) _returnvalue) "" (Utilities|String|ToString(Boolean) _output_get)))
  (bind _nextpointsindex (Default|GetNextPath (Variables|Default|GetGameModeRef) (LocalVariables|GetIsCrossRoad) _turndirection (.currentpath (Variables|Default|GetNewCurrentRegion))))
  (Development|PrintString (Utilities|String|Append "Right Now Direction:" (Utilities|String|EnumtoString _turndirection)))
  (CallFunction|SetCurrentRoad _nextpointsindex)
  (bind _targetpoints (Default|GetRegionTargetPoints (.Region (Utilities|Struct|BreakS_PlayerCurrentRegion (Variables|Default|GetNewCurrentRegion))) _nextpointsindex))
  (bind _output_get_2 (Variables|Default|SetTargetPoints _targetpoints))
  (Utilities|Array|RemoveIndex _output_get_2))

(fn Turn
  (params (direction :type E_Direction%20Enum :default "NewEnumerator0"))
  (bind _targetpoints (Variables|Default|GetTargetPoints))
  (if (<= (Math|Vector|Distance(Vector) (Transformation|GetActorLocation) (.Location (Utilities|Struct|BreakS_Point (Utilities|Array|Get(acopy) _targetpoints (- (Utilities|Array|Length _targetpoints) 1))))) 7.5e+02)
    (Variables|Default|SetTurnDirection direction)))

(fn UpdatePlayer0
  (params (delta%20Seconds :type Float%20%28double-precision%29))
  (LocalVariables|SetdeltaSeconds delta%20Seconds)
  (if (Utilities|IsValid (.Region (Utilities|Struct|BreakS_PlayerCurrentRegion (Variables|Default|GetNewCurrentRegion))))
    (if (Utilities|Array|IsEmpty (Variables|Default|GetTargetPoints))
      (if (Utilities|Enum|NotEqual(Enum) (Variables|/Game/Content/Blueprint/Game/BP_GameState.BP_GameState_C|GetPlayerStatus (Variables|Default|GetGameStateRef)) "NewEnumerator2")
        ;[1 1 1] Go to Next Region (or Path)
        (CallFunction|OnPassRegion)
        (else
          ;[1 1 1] Died
          (Variables|Default|SetCurrentRegion 0)
          (Variables|Default|SetNewCurrentRegion "")
          (Utilities|Array|Clear (Variables|Default|GetTargetPoints))
          (Development|PrintString "Died")))
      (else
        (LocalVariables|SetnexPoint (Utilities|Array|Get(acopy) (Variables|Default|GetTargetPoints)))
        (LocalVariables|SetStartPosition (Transformation|GetActorLocation))
        (LocalVariables|SetTargetPosition (+ (.Location (Utilities|Struct|BreakS_Point (LocalVariables|GetnexPoint))) "0.000000,0.000000,92.802551"))
        (LocalVariables|SetmoveDistance (Math|Vector|Distance(Vector) (LocalVariables|GetStartPosition) (LocalVariables|GetTargetPosition)))
        (LocalVariables|Setdirection (- (LocalVariables|GetTargetPosition) (Transformation|GetActorLocation)))
        (if (> (LocalVariables|GetmoveDistance) (* (LocalVariables|GetdeltaSeconds) (Variables|Default|Getspeed)))
          (CallFunction|CharactorMove (LocalVariables|GetdeltaSeconds) (LocalVariables|Getdirection) (Math|Rotator|FindLookatRotation (LocalVariables|GetStartPosition) (LocalVariables|GetTargetPosition)))
          (else
            (Utilities|Array|RemoveIndex (Variables|Default|GetTargetPoints))
            (Transformation|AddActorLocalRotation (Variables|Default|GetCharactor) false false)
            (Transformation|SetRelativeRotation (Variables|Character|GetMesh) "0.000000,-90.000000,0.000000" false false)))))))

(fn CharactorMove0
  (params (DeltaTime :type Float%20%28single-precision%29) (direction :type Vector) (rotator :type Rotator))
  (LocalVariables|Setdelta DeltaTime)
  (LocalVariables|SettargetDirection direction)
  (LocalVariables|SetlookAtRotator rotator)
  (Transformation|AddActorLocalOffset (* (Math|Vector|Normalize (LocalVariables|GettargetDirection)) (* (LocalVariables|Getdelta) (Variables|Default|Getspeed))) false false)
  (LocalVariables|SetActor%20Rotation (* (Transformation|GetActorRotation) -1.0))
  (Variables|Default|SetCharactor (Math|Rotator|CombineRotators (LocalVariables|GetlookAtRotator) (LocalVariables|GetActor%20Rotation)))
  (LocalVariables|SetMeshRotator (Math|Rotator|CombineRotators (LocalVariables|GetlookAtRotator) (* (Math|Rotator|CombineRotators (Transformation|GetWorldRotation (Variables|Character|GetMesh)) "0.000000,90.000000,0.000000") -1.0)))
  (if (>= (Math|Float|Absolute(Float) (.Yaw (Math|Rotator|BreakRotator (Variables|Default|GetCharactor)))) 1e+01)
    (Transformation|AddActorLocalRotation (Variables|Default|GetCharactor) false false)
    (Transformation|SetRelativeRotation (Variables|Character|GetMesh) "0.000000,-90.000000,0.000000" false false)
    (else
      (Transformation|AddLocalRotation (Variables|Character|GetMesh) (LocalVariables|GetMeshRotator) false false))))

(fn UpdatePlayer1
  (params (delta%20Seconds :type Float%20%28double-precision%29))
  (bind _targetpoints (Variables|Default|GetTargetPoints))
  (bind _output (Utilities|Array|Get(acopy) _targetpoints))
  (LocalVariables|SetdeltaSeconds delta%20Seconds)
  (LocalVariables|SetmoveDistance (* (LocalVariables|GetdeltaSeconds) (Variables|Default|Getspeed)))
  (if (Utilities|IsValid (.Region (Utilities|Struct|BreakS_PlayerCurrentRegion (Variables|Default|GetNewCurrentRegion))))
    (if (Utilities|Array|IsEmpty (Variables|Default|GetTargetPoints))
      (if (Utilities|Enum|NotEqual(Enum) (Variables|/Game/Content/Blueprint/Game/BP_GameState.BP_GameState_C|GetPlayerStatus (Variables|Default|GetGameStateRef)) "NewEnumerator2")
        ;[1 1 1] Go to Next Region (or Path)
        (CallFunction|OnPassRegion)
        (else
          ;[1 1 1] Died
          (Variables|Default|SetNewCurrentRegion "")
          (Utilities|Array|Clear (Variables|Default|GetTargetPoints))
          (Development|PrintString "Died")))
      (else
        (LocalVariables|SetnexPoint (Utilities|Array|Get(acopy) (Variables|Default|GetTargetPoints)))
        (bind _output_get (LocalVariables|SetStartPosition (Variables|Default|GetPlayerPosition)))
        (LocalVariables|SetTargetPosition (.Location (Utilities|Struct|BreakS_Point (LocalVariables|GetnexPoint))))
        (Development|PrintString (Utilities|String|Append "Start : " (Utilities|String|ToString(Vector) _output_get) " Target : " (Utilities|String|ToString(Vector) (.Location (Utilities|Struct|BreakS_Point (LocalVariables|GetnexPoint))))))
        (LocalVariables|SetDistance (Math|Vector|Distance(Vector) (LocalVariables|GetStartPosition) (LocalVariables|GetTargetPosition)))
        (LocalVariables|Setdirection (- (LocalVariables|GetTargetPosition) (LocalVariables|GetStartPosition)))
        (if (> (LocalVariables|GetDistance) (LocalVariables|GetmoveDistance))
          (CallFunction|CharactorMove1 (LocalVariables|GetdeltaSeconds) (LocalVariables|Getdirection) (Math|Rotator|FindLookatRotation (LocalVariables|GetStartPosition) (LocalVariables|GetTargetPosition)))
          (else
            (LocalVariables|SetpreviousPoint _output)
            (Development|PrintString (Utilities|String|ToString(Vector) (.Location (Utilities|Struct|BreakS_Point _output))))
            (Utilities|Array|RemoveIndex (Variables|Default|GetTargetPoints))
            (Transformation|AddActorLocalRotation (Variables|Default|GetCharactor) false false)
            (Transformation|SetRelativeRotation (Variables|Character|GetMesh) "0.000000,-90.000000,0.000000" false false)))))))

(fn CharactorMove1
  (params (DeltaTime :type Float%20%28single-precision%29) (direction :type Vector) (rotator :type Rotator))
  (LocalVariables|Setdelta DeltaTime)
  (LocalVariables|SettargetDirection direction)
  (LocalVariables|SetlookAtRotator rotator)
  (Transformation|AddActorLocalOffset (* (Math|Vector|Normalize (LocalVariables|GettargetDirection)) (* (LocalVariables|Getdelta) (Variables|Default|Getspeed))) false false)
  (bind _output_get (Variables|Default|SetPlayerPosition (+ (Variables|Default|GetPlayerPosition) (* (Math|Vector|Normalize (LocalVariables|GettargetDirection)) (* (LocalVariables|Getdelta) (Variables|Default|Getspeed))))))
  (LocalVariables|SetActor%20Rotation (* (Transformation|GetActorRotation) -1.0))
  (Variables|Default|SetCharactor (Math|Rotator|CombineRotators (LocalVariables|GetlookAtRotator) (LocalVariables|GetActor%20Rotation)))
  (LocalVariables|SetMeshRotator (Math|Rotator|CombineRotators (LocalVariables|GetlookAtRotator) (* (Math|Rotator|CombineRotators (Transformation|GetWorldRotation (Variables|Character|GetMesh)) "0.000000,90.000000,0.000000") -1.0)))
  (if (>= (Math|Float|Absolute(Float) (.Yaw (Math|Rotator|BreakRotator (Variables|Default|GetCharactor)))) 5.0)
    (Transformation|AddActorLocalRotation (Variables|Default|GetCharactor) false false)
    (Transformation|SetRelativeRotation (Variables|Character|GetMesh) "0.000000,-90.000000,0.000000" false false)
    (else
      (Transformation|AddLocalRotation (Variables|Character|GetMesh) (LocalVariables|GetMeshRotator) false false))))