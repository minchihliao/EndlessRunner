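; Base road actor for courses that builds road geometry from a spline and serves waypoints along it.
; Construction adds two spline meshes per Spline segment: the road and a narrow, slightly raised line.
; BeginPlay caches world location and tangent rotation per spline component, skipping first points, and maps additional splines to direction regions by index.
; Helper functions read those points like a queue via a shared position index, with debug prints.
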(event EventBeginPlay
  (CallFunction|SetAllPoints))

(event Collision|EventActorBeginOverlap
  (params (OtherActor :type Actor%20Object%20Reference)))

(event EventTick
  (params (DeltaSeconds :type Float%20%28single-precision%29)))

(fn ConstructionScript
  (CallFunction|SpawnRoadMesh (Variables|Default|GetSpline)))

(fn SpawnRoadMesh
  (params (spline :type Spline%20Component%20Object%20Reference))
  (LocalVariables|SettargetSpline spline)
  (for _index (range 0 (- (Spline|GetNumberOfSplinePoints spline) 2))
    (bind _returnvalue (AddComponent|AddSplineMeshComponent false (Math|Transform|MakeTransform "0, 0, 0" (Transformation|GetActorRotation) "1.000000,1.000000,1.000000")))
    (Transformation|SetWorldRotation _returnvalue (Math|Rotator|MakeRotator 0.0 0.0 0.0) false false)
    (Collision|SetCollisionEnabled _returnvalue "QueryAndPhysics")
    (Transformation|AttachComponentToComponent _returnvalue (Variables|Default|GetDefaultSceneRoot) "None" "KeepRelative" "KeepRelative" "KeepRelative" true)
    (SplineMesh|SetStartandEnd _returnvalue (+ (- (Transformation|GetWorldLocation (LocalVariables|GettargetSpline)) (Transformation|GetActorLocation)) (.Location (Spline|GetLocationandTangentatSplinePoint (LocalVariables|GettargetSpline) _index "Local"))) (.Tangent (Spline|GetLocationandTangentatSplinePoint (LocalVariables|GettargetSpline) _index "Local")) (+ (.Location (Spline|GetLocationandTangentatSplinePoint (LocalVariables|GettargetSpline) (+ _index 1) "Local")) (- (Transformation|GetWorldLocation (LocalVariables|GettargetSpline)) (Transformation|GetActorLocation))) (.Tangent (Spline|GetLocationandTangentatSplinePoint (LocalVariables|GettargetSpline) (+ _index 1) "Local")) true :!class /Script/Engine.SplineMeshComponent)
    (bind _returnvalue_2 (AddComponent|AddSplineMeshComponent false))
    (Collision|SetCollisionEnabled _returnvalue_2 "QueryAndPhysics")
    (Transformation|AttachComponentToComponent _returnvalue_2 (Variables|Default|GetDefaultSceneRoot) "None" "KeepRelative" "KeepRelative" "KeepRelative" true)
    (LocalVariables|SetSpwanLineCurPoint (Utilities|Struct|MakeS_Point (+ (Math|Vector|MakeVector (.x (.Location (Spline|GetLocationandTangentatSplinePoint (LocalVariables|GettargetSpline) _index "Local"))) (.y (.Location (Spline|GetLocationandTangentatSplinePoint (LocalVariables|GettargetSpline) _index "Local"))) (+ (.z (.Location (Spline|GetLocationandTangentatSplinePoint (LocalVariables|GettargetSpline) _index "Local"))) 2.5)) (- (Transformation|GetWorldLocation (LocalVariables|GettargetSpline)) (Transformation|GetActorLocation))) (Math|Conversions|RotationFromXVector (.Tangent (Spline|GetLocationandTangentatSplinePoint (LocalVariables|GettargetSpline) _index "Local")))))
    (LocalVariables|SetSpwanLineNextPoint (Utilities|Struct|MakeS_Point (+ (Math|Vector|MakeVector (.x (.Location (Spline|GetLocationandTangentatSplinePoint (LocalVariables|GettargetSpline) (+ _index 1) "Local"))) (.y (.Location (Spline|GetLocationandTangentatSplinePoint (LocalVariables|GettargetSpline) (+ _index 1) "Local"))) (+ (.z (.Location (Spline|GetLocationandTangentatSplinePoint (LocalVariables|GettargetSpline) (+ _index 1) "Local"))) 2.5)) (- (Transformation|GetWorldLocation (LocalVariables|GettargetSpline)) (Transformation|GetActorLocation))) (Math|Conversions|RotationFromXVector (.Tangent (Spline|GetLocationandTangentatSplinePoint (LocalVariables|GettargetSpline) (+ _index 1) "Local")))))
    (SplineMesh|SetStartandEnd _returnvalue_2 (.location (LocalVariables|GetSpwanLineCurPoint)) (Math|Rotator|GetRotationXVector (.rotator (LocalVariables|GetSpwanLineCurPoint))) (.location (LocalVariables|GetSpwanLineNextPoint)) (Math|Rotator|GetRotationXVector (.rotator (LocalVariables|GetSpwanLineNextPoint))) true :!class /Script/Engine.SplineMeshComponent)
    (SplineMesh|SetStartScale _returnvalue_2 "(X=0.200000,Y=0.200000)" true :!class /Script/Engine.SplineMeshComponent)
    (SplineMesh|SetEndScale _returnvalue_2 "(X=0.200000,Y=0.200000)" true :!class /Script/Engine.SplineMeshComponent)))

(fn IsPointsEmpty
  (params (SplineIndex :type Integer))
  (return (>= (Variables|Default|GetSplinePositionIndex) (Utilities|Array|Length (Utilities|Struct|BreakS_AllRegionPoints (Utilities|Array|Get(acopy) (Variables|Default|GetAllPoints) SplineIndex))))))

(fn GetNextPoint
  (params (SplineIndex :type Integer))
  (return (Utilities|Array|Get(acopy) (Utilities|Struct|BreakS_AllRegionPoints (Utilities|Array|Get(acopy) (Variables|Default|GetAllPoints) SplineIndex)) (Variables|Default|GetSplinePositionIndex))))

(fn DequeuePoints
  (Math|Integer|IncrementInt (Variables|Default|GetSplinePositionIndex)
    (:%20%20
      (return))))

(fn GetRegionTargetPoints
  (params (index :type E_Direction%20Enum :default "NewEnumerator0"))
  (bind _returnvalue (Math|Conversions|ToInteger(Byte) index))
  (bind _allpoints (Variables|Default|GetAllPoints))
  (bind _output (Utilities|Array|Get(acopy) _allpoints _returnvalue))
  (bind _points (Utilities|Struct|BreakS_AllRegionPoints _output))
  (for _array_element _points
    (Development|PrintString (Utilities|String|ToString(Vector) (.Location (Utilities|Struct|BreakS_Point _array_element)))))
  (return _points))

(fn IsNextRegionExist
  (return (== (Utilities|Array|IsEmpty (Variables|Default|GetRegion)) false)))

(fn SetAllPoints
  (bind _points (Variables|Default|GetPoints))
  (Utilities|Array|Clear (Variables|Default|GetAllPoints))
  (Utilities|Array|Clear (Variables|Default|GetPoints))
  (for (_array_element _array_index) (Actor|GetComponentsByClass "/Script/Engine.SplineComponent")
    (for _index (range 1 (- (Spline|GetNumberOfSplinePoints _array_element) 1))
      (Utilities|Array|Add (Variables|Default|GetPoints) (Utilities|Struct|MakeS_Point (.Location (Spline|GetLocationandTangentatSplinePoint _array_element _index "World")) (Math|Conversions|RotationFromXVector (.Tangent (Spline|GetLocationandTangentatSplinePoint _array_element _index "World")))))
      (Development|PrintString (Utilities|String|Append (Utilities|GetObjectName _array_element) (Utilities|String|ToString(Vector) (.Location (Spline|GetLocationandTangentatSplinePoint _array_element _index "World"))))))
    (Utilities|Array|Add (Variables|Default|GetAllPoints) (Utilities|Struct|MakeS_AllRegionPoints _points))
    (Utilities|Array|Clear _points)
    (if (!= _array_index 0)
      (Utilities|Array|Add (Variables|Default|GetRegion) (Utilities|Enum|ByteToEnumE_Direction (Math|Conversions|ToByte(Integer) _array_index)))))
  (for _array_element_2 (Variables|Default|GetRegion)
    (Development|PrintString (Utilities|String|EnumtoString _array_element_2))))